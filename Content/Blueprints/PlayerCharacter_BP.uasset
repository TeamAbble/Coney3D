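; Player character Blueprint that sets up its player's lobby/pause menu and HUD and caches camera, weapon and aim references.
; On possession it derives PlayerIndex from its position among all PlayerCharacter_BP actors, then creates both widgets for that controller.
; The pause input toggles the menu, input mode, cursor, HUD and GamePaused flag.
; Tick polls health to refresh the HUD bar; music and host/join widget nodes are disconnected.
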(event `EnhancedInput|/Game/ThirdPerson/Input/Actions/IA_PauseMenu`
  (params (ActionValue :type Boolean) (ElapsedSeconds :type "Float (double-precision)") (TriggeredSeconds :type "Float (double-precision)") (InputAction :type "InputAction Object Reference" :default "/Game/ThirdPerson/Input/Actions/IA_PauseMenu.IA_PauseMenu"))
  (:`Triggered`
    (bind _output_get (set `self.IsMainMenuOpen` (not (`self.IsMainMenuOpen`))))
    (`self.OpenPauseMenu` _output_get)))

(event `self.ReceivePossessed`
  (params (NewController :type "Controller Object Reference"))
  (`self.AssignPlayerIndex`)
  (bind _returnvalue (`|CreateWidget` "/Game/UI/WB_Lobby.WB_Lobby_C" (`GameplayStatics.GetPlayerController` (`self.PlayerIndex`))))
  (bind _output_get (set `self.WB_Lobby` _returnvalue))
  (set `/Game/UI/WB_Lobby.Player` self _output_get)
  (`UserWidget.AddToViewport` _output_get 0)
  (`Widget.SetVisibility` _output_get "Hidden")
  (`Widget.SetIsEnabled` _output_get false)
  (bind _returnvalue_2 (`|CreateWidget` "/Game/UI/WB_PIZZAHUD.WB_PIZZAHUD_C" (`GameplayStatics.GetPlayerController` (`self.PlayerIndex`))))
  (bind _output_get_2 (set `self.WB HUD` _returnvalue_2))
  (`UserWidget.AddToPlayerScreen` _output_get_2 0))

(event `self.ReceiveTick`
  (params (DeltaSeconds :type "Float (single-precision)"))
  (bind _returnvalue (`self.GetCurrentHealth`))
  (if (!= (`self._health`) (`self.GetCurrentHealth`))
    (`ProgressBar.SetPercent` (`/Game/UI/WB_PIZZAHUD.HealthBar` (`self.WB HUD`)) (/ _returnvalue (`self.GetMaxHealth`)))
    (bind _output_get (set `self._health` _returnvalue))
    (`KismetSystemLibrary.PrintString` (`KismetStringLibrary.BuildString_Double` "Updated Health to " "" _output_get))))

(fn `AssignPlayerIndex`
  (bind _outactors (`GameplayStatics.GetAllActorsOfClass` "PlayerCharacter_BP_C"))
  (for (_array_element _array_index) _outactors
    (if (== _array_element self)
      (set `self.PlayerIndex` _array_index)
      (break))))

(fn `OpenPauseMenu`
  (params (Pause :type Boolean))
  (bind _ismainmenuopen (`self.IsMainMenuOpen`))
  (bind _wb_hud (`self.WB HUD`))
  (bind _returnvalue (`GameplayStatics.GetPlayerController` (`self.PlayerIndex`)))
  (bind _output_get (set `self.IsMainMenuOpen` Pause))
  (if _output_get
    (`Widget.SetVisibility` (`self.WB_Lobby`) "Visible")
    (`Widget.SetIsEnabled` (`self.WB_Lobby`) true)
    (`WidgetBlueprintLibrary.SetInputMode_UIOnlyEx` _returnvalue (`self.WB_Lobby`))
    (else
      (`/Game/UI/WB_Lobby.ResetPause` (`self.WB_Lobby`))
      (`Widget.SetVisibility` (`self.WB_Lobby`) "Hidden")
      (`Widget.SetIsEnabled` (`self.WB_Lobby`) false)
      (`WidgetBlueprintLibrary.SetInputMode_GameOnly` _returnvalue)))
  (set `PlayerController.bShowMouseCursor` (`self.IsMainMenuOpen`) (`GameplayStatics.GetPlayerController` (`self.PlayerIndex`)))
  (set `self.GamePaused` _ismainmenuopen)
  (if (`KismetSystemLibrary.IsValid` (`self.WB HUD`))
    (if _ismainmenuopen
      (`Widget.SetVisibility` _wb_hud "Hidden")
      (else
        (`Widget.SetVisibility` _wb_hud "Visible")))))

(fn `UserConstructionScript`
  (bind _tpcam (`self.TPCam`))
  (set `self.weaponPointRef` (`self.WeaponPoint`))
  (set `self.playerCam` (`self.TPCam`))
  (set `self.aimRef` (`self.AimRefPoint`))
  (set `self.firstPersonCamera` (`self.FPCam`))
  (set `self.thirdPersonCamera` _tpcam)
  (set `self.startFOV` (`CameraComponent.FieldOfView` _tpcam)))